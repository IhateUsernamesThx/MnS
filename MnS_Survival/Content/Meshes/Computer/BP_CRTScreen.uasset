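; BP_CRTScreen is a computer CRT screen that shows a widget's rendered output on a static mesh.
; On BeginPlay it creates a dynamic instance of M_CRTScreen on one of the mesh's material slots.
; Every Tick it feeds the Widget's render target into that material's texture parameter.
; DoInteract shows the mouse cursor and switches the first player controller to UI-only input, with no path back in this Blueprint.
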(event EventBeginPlay
  (bind _returnvalue (Rendering|Material|CreateDynamicMaterialInstance (Variables|Default|GetStaticMesh) 1 "/Game/Meshes/Computer/M_CRTScreen.M_CRTScreen" "None" :!class /Script/Engine.PrimitiveComponent))
  (Variables|Default|SetDMI _returnvalue))

(event EventDoInteract
  (bind _returnvalue (Game|GetPlayerController 0))
  (Variables|/Script/Engine.PlayerController|SetbShowMouseCursor _returnvalue true)
  (Input|SetInputModeUIOnly _returnvalue 0 "DoNotLock" false))

(event EventTick
  (params (DeltaSeconds :type Float%20%28single-precision%29))
  (Rendering|Material|SetTextureParameterValue (Variables|Default|GetDMI) "Tex" (Class|WidgetComponent|GetRenderTarget (Variables|Default|GetWidget))))

(fn ConstructionScript)