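; BP_Fatigue is a self-contained, temporary debuff actor that fatigues the first-person player character while it exists.
; On BeginPlay it disables sprinting, halves jump velocity and adds a move modifier through the character's ACPlayerStats component.
; A timer, set to loop, calls FatigueEnd after a fixed delay, which reverses all three changes and destroys the actor, so it fires only once.
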(event Custom|FatigueEnd
  (Variables|/Script/Engine.CharacterMovementComponent|SetJumpZVelocity (Variables|/Script/Engine.Character|GetCharacterMovement (stale EventBeginPlay _output_get)) (* (Variables|/Script/Engine.CharacterMovementComponent|GetJumpZVelocity (Variables|/Script/Engine.Character|GetCharacterMovement (stale EventBeginPlay _output_get))) 2.0))
  (Default|RemoveMoveModifier (Variables|Default|GetAC%20Player%20Stats) 0.5 "NewEnumerator1")
  (Actor|DestroyActor)
  (Variables|/Game/FirstPerson/Blueprints/BP_FirstPersonCharacter.BP_FirstPersonCharacter_C|SetCanSprinting (Variables|Default|GetAs%20BP%20First%20Person%20Character) true))

(event EventBeginPlay
  (bind _asbp_first_person_character (Utilities|Casting|CastToBP_FirstPersonCharacter (Game|GetPlayerCharacter 0)))
  (bind _output_get (Variables|Default|SetAs%20BP%20First%20Person%20Character _asbp_first_person_character))
  (Variables|/Game/FirstPerson/Blueprints/BP_FirstPersonCharacter.BP_FirstPersonCharacter_C|SetCanSprinting _output_get false)
  (Variables|Default|SetAC%20Player%20Stats (Variables|/Game/FirstPerson/Blueprints/BP_FirstPersonCharacter.BP_FirstPersonCharacter_C|GetAC_PlayerStats _output_get))
  (Utilities|Time|SetTimerbyEvent (delegate Custom|FatigueEnd) 1e+01 true)
  (Variables|/Script/Engine.CharacterMovementComponent|SetJumpZVelocity (Variables|/Script/Engine.Character|GetCharacterMovement _output_get) (/ (Variables|/Script/Engine.CharacterMovementComponent|GetJumpZVelocity (Variables|/Script/Engine.Character|GetCharacterMovement _output_get)) 2.0))
  (Default|AddMoveModifier (Variables|Default|GetAC%20Player%20Stats) 0.5 "NewEnumerator1"))

(fn ConstructionScript)