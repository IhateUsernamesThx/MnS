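; BP_DamagePlayer is an effect actor that damages the player as soon as it begins play.
; It casts player 0's character to BP_FirstPersonCharacter and passes EffectMagnitude to ReceiveDamage on that character's ACPlayerStats component.
; It then plays a 2D hit sound with slight random pitch variation.
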(event EventBeginPlay
  (|CallParentFunction)
  (bind _asbp_first_person_character (Utilities|Casting|CastToBP_FirstPersonCharacter (Game|GetPlayerCharacter 0)))
  (bind _output_get (Variables|Default|SetAC%20Player%20Stats (Variables|/Game/FirstPerson/Blueprints/BP_FirstPersonCharacter.BP_FirstPersonCharacter_C|GetAC_PlayerStats _asbp_first_person_character)))
  (Default|ReceiveDamage _output_get (Variables|Default|GetEffectMagnitude))
  (Audio|PlaySound2D "/Game/Audio/RecieveDamage_01.RecieveDamage_01" 0.4 (Math|Random|RandomFloatinRange 0.95 1.05) 0.2 0 0))

(event Collision|EventActorBeginOverlap
  (params (OtherActor :type Actor%20Object%20Reference))
  (|CallParentFunction OtherActor) ; This node is disabled and will not be called.\nDrag off pins to build functionality.
)

(event EventTick
  (params (DeltaSeconds :type Float%20%28single-precision%29))
  (|CallParentFunction DeltaSeconds) ; This node is disabled and will not be called.\nDrag off pins to build functionality.
)

(fn ConstructionScript
  (|CallParentFunction))