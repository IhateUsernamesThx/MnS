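; Effect actor that gives the first-person player a new data log entry as soon as it begins play.
; On BeginPlay it checks the player's Logs for the entry, also matching a copy with NewLog cleared to avoid duplicates.
; A missing entry is inserted at the front, then the actor destroys itself and notifies the player stats HUD and scanned log widget.
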(event EventBeginPlay
  (bind _datalogentry (Variables|Default|GetDataLogEntry))
  (bind (_sender _bodytext) (Utilities|Struct|BreakF_DataLog _datalogentry))
  (|CallParentFunction)
  (bind _asbp_first_person_character (Utilities|Casting|CastToBP_FirstPersonCharacter (Game|GetPlayerCharacter 0)))
  (if (not (or (Utilities|Array|ContainsItem (Variables|/Game/FirstPerson/Blueprints/BP_FirstPersonCharacter.BP_FirstPersonCharacter_C|GetLogs _asbp_first_person_character) (Variables|Default|GetDataLogEntry)) (Utilities|Array|ContainsItem (Variables|/Game/FirstPerson/Blueprints/BP_FirstPersonCharacter.BP_FirstPersonCharacter_C|GetLogs _asbp_first_person_character) (Utilities|Struct|MakeF_DataLog _sender _bodytext false))))
    (Utilities|Array|Insert (Variables|/Game/FirstPerson/Blueprints/BP_FirstPersonCharacter.BP_FirstPersonCharacter_C|GetLogs _asbp_first_person_character) (Variables|Default|GetDataLogEntry))
    (Actor|DestroyActor)
    (Default|RecievedMessage (Variables|/Game/UI/WB_HUD.WB_HUD_C|GetWB_PlayerStats (Variables|/Game/FirstPerson/Blueprints/BP_FirstPersonCharacter.BP_FirstPersonCharacter_C|GetHUD _asbp_first_person_character)) true)
    (Default|LetterRecieved (Variables|/Game/FirstPerson/Blueprints/BP_FirstPersonCharacter.BP_FirstPersonCharacter_C|GetScannedLogWidget _asbp_first_person_character))))

(event Collision|EventActorBeginOverlap
  (params (OtherActor :type Actor%20Object%20Reference))
  (|CallParentFunction OtherActor) ; This node is disabled and will not be called.\nDrag off pins to build functionality.
)

(event EventTick
  (params (DeltaSeconds :type Float%20%28single-precision%29))
  (|CallParentFunction DeltaSeconds) ; This node is disabled and will not be called.\nDrag off pins to build functionality.
)

(fn ConstructionScript
  (|CallParentFunction))