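; Effect actor that plays a harvest animation montage on its owner's skeletal mesh.
; On BeginPlay it gets the mesh from the owner's ReturnScanDataMessage, casts it to a skeletal mesh component and plays HarvestAnimation on it.
; It destroys itself when the montage completes or blends out, but stays alive if the cast fails.
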(event EventBeginPlay
  (bind _mesh (Class|BPIScanData|ReturnScanData(Message) (Components|GetOwner)))
  (bind _asskeletal_mesh_component (Utilities|Casting|CastToSkeletalMeshComponent _mesh))
  (Animation|Montage|PlayMontage _asskeletal_mesh_component (Variables|Default|GetHarvestAnimation)
    (:OnCompleted
      _)
    (:OnBlendOut
      _))
  (Actor|DestroyActor))

(event Collision|EventActorBeginOverlap
  (params (OtherActor :type Actor%20Object%20Reference))
  (|CallParentFunction OtherActor) ; This node is disabled and will not be called.\nDrag off pins to build functionality.
)

(event EventTick
  (params (DeltaSeconds :type Float%20%28single-precision%29))
  (|CallParentFunction DeltaSeconds) ; This node is disabled and will not be called.\nDrag off pins to build functionality.
)

(fn ConstructionScript
  (|CallParentFunction))