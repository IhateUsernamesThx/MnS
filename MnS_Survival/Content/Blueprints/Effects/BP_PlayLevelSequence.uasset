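; Effect actor that plays a death level sequence for the scannable skeleton that owns it.
; On BeginPlay it creates a sequence player and binds the owner, cast to BP_ScannableSkeletonBase, in place of the asset's own binding.
; It overrides instance data so the sequence's transform origin follows the owner, using its actor reference plus a transform of X/Y location and yaw, then plays.
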(event EventBeginPlay
  (bind _returnvalue (Components|GetOwner))
  (bind _returnvalue_2 (Transformation|GetActorLocation _returnvalue))
  (|CallParentFunction)
  (bind (_outactor _returnvalue_3) (Sequencer|Player|CreateLevelSequencePlayer (Variables|Default|GetDeath%20Sequence)))
  (bind _asbp_scannable_skeleton_base (Utilities|Casting|CastToBP_ScannableSkeletonBase (Components|GetOwner)))
  (Class|LevelSequenceActor|AddBinding _outactor (|GetSequenceBinding) _asbp_scannable_skeleton_base false)
  (Variables|/Script/LevelSequence.LevelSequenceActor|SetbOverrideInstanceData _outactor true)
  (bind _asdefault_level_sequence_instance_data (Utilities|Casting|CastToDefaultLevelSequenceInstanceData (Variables|/Script/LevelSequence.LevelSequenceActor|GetDefaultInstanceData _outactor)))
  (Variables|/Script/LevelSequence.DefaultLevelSequenceInstanceData|SetTransformOriginActor _asdefault_level_sequence_instance_data _returnvalue)
  (Variables|/Script/LevelSequence.DefaultLevelSequenceInstanceData|SetTransformOrigin _asdefault_level_sequence_instance_data (Math|Transform|MakeTransform (Math|Vector|MakeVector (.x _returnvalue_2) (.y _returnvalue_2) 0.0) (Math|Rotator|MakeRotator 0.0 0.0 (.yaw (Transformation|GetActorRotation _returnvalue)))))
  (Sequencer|Player|Play _returnvalue_3 :!class /Script/MovieScene.MovieSceneSequencePlayer))

(event Collision|EventActorBeginOverlap
  (params (OtherActor :type Actor%20Object%20Reference))
  (|CallParentFunction OtherActor) ; This node is disabled and will not be called.\nDrag off pins to build functionality.
)

(event EventTick
  (params (DeltaSeconds :type Float%20%28single-precision%29))
  (|CallParentFunction DeltaSeconds) ; This node is disabled and will not be called.\nDrag off pins to build functionality.
)

(fn ConstructionScript
  (|CallParentFunction))