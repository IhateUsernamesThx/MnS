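; BP_EffectPoison is a poison effect actor that deals damage over time to the player.
; On BeginPlay it caches the ACPlayerStats component of the first-person character, then starts a looping one-second damage timer and a timer for the effect duration.
; Each tick passes base damage scaled by effect magnitude to ReceiveDamage, and the actor destroys itself when the duration ends.
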(event Custom|EndEffect
  (Actor|DestroyActor))

(event Custom|DamageTick
  (Default|ReceiveDamage (stale EventBeginPlay _output_get) (* (Variables|Default|GetBaseDamage) (Variables|Default|GetEffectMagnitude))))

(event EventBeginPlay
  (bind _asbp_first_person_character (Utilities|Casting|CastToBP_FirstPersonCharacter (Game|GetPlayerCharacter 0)))
  (bind _output_get (Variables|Default|SetAC%20Player%20Stats (Variables|/Game/FirstPerson/Blueprints/BP_FirstPersonCharacter.BP_FirstPersonCharacter_C|GetAC_PlayerStats _asbp_first_person_character)))
  (Utilities|Time|SetTimerbyEvent (delegate Custom|DamageTick) 1.0 true)
  (Utilities|Time|SetTimerbyEvent (delegate Custom|EndEffect) (Variables|Default|GetEffectDuration)))

(fn ConstructionScript
  (|CallParentFunction))