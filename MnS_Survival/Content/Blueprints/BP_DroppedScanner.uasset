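; A dropped scanner that the player interacts with to collect the data entries stored on it.
; DoInteract puts each StoredNewData entry missing from the first-person character's NewDataEntries at the front of that list, plays a pop sound, then destroys itself and its waypoint.
; ReturnScanData exposes its scan data and mesh, always reporting it as unscanned.
; A line trace that would snap it to the surface below and align it to the normal is never run.
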(event EventBeginPlay)

(event EventDoInteract
  (bind _asbp_first_person_character (Utilities|Casting|CastToBP_FirstPersonCharacter (Game|GetPlayerCharacter 0)))
  (for _array_element (Variables|Default|GetStoredNewData)
    (if (not (Utilities|Array|ContainsItem (Variables|/Game/FirstPerson/Blueprints/BP_FirstPersonCharacter.BP_FirstPersonCharacter_C|GetNewDataEntries _asbp_first_person_character) _array_element))
      (Utilities|Array|Insert (Variables|/Game/FirstPerson/Blueprints/BP_FirstPersonCharacter.BP_FirstPersonCharacter_C|GetNewDataEntries _asbp_first_person_character) _array_element)))
  (Audio|PlaySoundatLocation "/Game/Audio/67088__sunnysidesound__pop_2.67088__sunnysidesound__pop_2" (Transformation|GetWorldLocation (Variables|Default|GetStaticMesh)) "0, 0, 0" 1.0 1.0 0.0 0 0 0 0)
  (Actor|DestroyActor)
  (Actor|DestroyActor (Variables|Default|GetWaypoint)))

(fn ConstructionScript)

(fn ReturnScanData
  (return (Variables|Default|GetScan%20Data) (Variables|Default|GetStaticMesh) false))