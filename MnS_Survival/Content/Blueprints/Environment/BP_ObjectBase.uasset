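; BP_ObjectBase is a base environment object that can be interacted with and scanned, driven by a Definition.
; The construction script applies the Definition's mesh.
; Interaction executes each of the Definition's gameplay effects with a context naming the interacting actor as instigator and itself as owner.
; It stores a scanned flag and returns it with the mesh and scan data built from the Definition's name, description, type and category.
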(event EventSetScanData
  (params (Scanned :type Boolean))
  (Variables|Default|SetScanned Scanned))

(event EventDoInteract
  (params (InteractingActor :type Actor%20Object%20Reference))
  (for _array_element (Variables|/Game/Blueprints/Environment/PDA_ObjectDefinition.PDA_ObjectDefinition_C|GetGameplayEffects (Variables|Default|GetDefinition))
    (Class|GameplayEffect|Execute _array_element (Utilities|Struct|MakeInteractionContext InteractingActor self))))

(fn ConstructionScript
  (Components|StaticMesh|SetStaticMesh (Variables|Default|GetMesh) (Variables|/Game/Blueprints/Environment/PDA_ObjectDefinition.PDA_ObjectDefinition_C|GetMesh (Variables|Default|GetDefinition))))

(fn ReturnScanData
  (bind _definition (Variables|Default|GetDefinition))
  (bind _name (Variables|/Game/Blueprints/Environment/PDA_ObjectDefinition.PDA_ObjectDefinition_C|GetName _definition))
  (return (Utilities|Struct|MakeF_ScannableData _name _name (Variables|/Game/Blueprints/Environment/PDA_ObjectDefinition.PDA_ObjectDefinition_C|GetDescription _definition) (Variables|/Game/Blueprints/Environment/PDA_ObjectDefinition.PDA_ObjectDefinition_C|GetObjectType _definition) (Variables|/Game/Blueprints/Environment/PDA_ObjectDefinition.PDA_ObjectDefinition_C|GetObjectCategory _definition)) (Variables|Default|GetMesh) (Variables|Default|GetScanned)))