(event OnComponentBeginOverlap(HearingDetection)
  (params (OverlappedComponent :type Primitive%20Component%20Object%20Reference) (OtherActor :type Actor%20Object%20Reference) (OtherComp :type Primitive%20Component%20Object%20Reference) (OtherBodyIndex :type Integer) (bFromSweep :type Boolean) (SweepResult :type Hit%20Result%20Structure%20%28by%20ref%29))
  (bind _asbp_character (Utilities|Casting|CastToBP_Character OtherActor))
  (if (AI|Components|NavMovement|IsCrouching (Variables|/Script/Engine.Character|GetCharacterMovement _asbp_character))
    (bind _returnvalue (Utilities|Time|SetTimerbyEvent (delegate Custom|Checking) 0.01 true))
    (else
      (Development|PrintString "I hear you"))))

(event OnComponentBeginOverlap(CrouchedDetection)
  (params (OverlappedComponent :type Primitive%20Component%20Object%20Reference) (OtherActor :type Actor%20Object%20Reference) (OtherComp :type Primitive%20Component%20Object%20Reference) (OtherBodyIndex :type Integer) (bFromSweep :type Boolean) (SweepResult :type Hit%20Result%20Structure%20%28by%20ref%29))
  (Utilities|Casting|CastToBP_Character OtherActor)
  (Development|PrintString "I smell you"))

(event OnComponentEndOverlap(HearingDetection)
  (params (OverlappedComponent :type Primitive%20Component%20Object%20Reference) (OtherActor :type Actor%20Object%20Reference) (OtherComp :type Primitive%20Component%20Object%20Reference) (OtherBodyIndex :type Integer))
  (Utilities|Time|ClearandInvalidateTimerbyHandle (stale OnComponentBeginOverlap(HearingDetection) _returnvalue)))

(event Custom|Checking
  (bind _asbp_character (Utilities|Casting|CastToBP_Character (stale OnComponentBeginOverlap(HearingDetection) OtherActor)))
  (if (AI|Components|NavMovement|IsCrouching (Variables|/Script/Engine.Character|GetCharacterMovement _asbp_character))
    (bind _returnvalue (Utilities|Time|SetTimerbyEvent (delegate Custom|Checking) 0.01 true))
    (else
      (Development|PrintString "I hear you"))))

(fn ConstructionScript)