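; Player stats component managing health, O2, skill EXP and walk speed, and creating the leveling menu.
; A looping timer drains O2, then health when empty, updating HUD bars; temporary consumption multipliers change its rate until a capped recovery timer resets them.
; AddExp recursively levels skills against DT_LevelExp thresholds.
; Move modifiers, mapped by value, apply additions before multipliers to MaxWalkSpeed; Dead is an empty stub.
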(event Custom|UpdateO2Tick
  (Utilities|Time|ClearandInvalidateTimerbyHandle (Variables|Default|GetO2TickTimer))
  (bind _returnvalue (Utilities|Time|SetTimerbyFunctionName 0 "O2Tick" (/ 2.0 (Variables|Default|GetO2ConsumptionMultiplier)) true))
  (Variables|Default|SetO2TickTimer _returnvalue))

(event Custom|O2ConsumptionRecovery
  (params (O2ConsumptionMultiplier :type Float%20%28double-precision%29) (RecoveryTime :type Float%20%28single-precision%29))
  (Variables|Default|SetO2ConsumptionMultiplier O2ConsumptionMultiplier)
  (CallFunction|UpdateO2Tick)
  (if (Utilities|Time|IsValidTimerHandle (Variables|Default|GetO2RecoveryTimer))
    (bind _returnvalue (Utilities|Time|SetTimerbyEvent (EventDispatchers|CreateEvent :!event Custom|O2RecoveryEnd) (Math|Float|Clamp(Float) (+ (Utilities|Time|GetTimerRemainingTimebyHandle (Variables|Default|GetO2RecoveryTimer)) RecoveryTime) 0.0 5.0)))
    (Utilities|Time|ClearandInvalidateTimerbyHandle (Variables|Default|GetO2RecoveryTimer))
    (Variables|Default|SetO2RecoveryTimer _returnvalue)
    (else
      (bind _returnvalue_2 (Utilities|Time|SetTimerbyEvent (EventDispatchers|CreateEvent :!event Custom|O2RecoveryEnd) (Math|Float|Clamp(Float) RecoveryTime 0.0 5.0)))
      (Variables|Default|SetO2RecoveryTimer _returnvalue_2))))

(event Custom|O2RecoveryEnd
  (Utilities|Time|ClearandInvalidateTimerbyHandle (Variables|Default|GetO2RecoveryTimer))
  (Variables|Default|SetO2ConsumptionMultiplier 1.0)
  (CallFunction|UpdateO2Tick))

(event EventBeginPlay
  (bind _asbp_first_person_character (Utilities|Casting|CastToBP_FirstPersonCharacter (Game|GetPlayerCharacter 0)))
  (Variables|Default|SetAs%20BP%20First%20Person%20Character _asbp_first_person_character)
  (bind _output_get (Variables|Default|SetPlayerNumber (Utilities|Text|FormatText "#{0}" (Utilities|Text|ToText(Integer) (Math|Random|RandomIntegerinRange 0 9999) false false))))
  (bind _returnvalue (UserInterface|CreateWidget "/Game/UI/WB_LevelingMenu.WB_LevelingMenu_C" 0 _output_get))
  (Variables|Default|SetLevelMenu _returnvalue)
  (bind _returnvalue_2 (Utilities|Time|SetTimerbyFunctionName 0 "O2Tick" (/ 2.0 (Variables|Default|GetO2ConsumptionMultiplier)) true))
  (Variables|Default|SetO2TickTimer _returnvalue_2))

(fn ReceiveDamage
  (params (IncomingDamage :type Float%20%28double-precision%29))
  (Variables|Default|SetCurrentHealth (- (Variables|Default|GetCurrentHealth) IncomingDamage))
  (CallFunction|DeathCheck 0.0)
  (CallFunction|SetStatPercentage (Variables|/Game/UI/WB_PlayerStats.WB_PlayerStats_C|GetPB_Health (Variables|Default|GetWB%20Player%20Stats)) (Variables|Default|GetCurrentHealth) (Variables|Default|GetMaxHealth)))

(fn DeathCheck
  (params (CurrentHealth :type Float%20%28double-precision%29))
  (if (<= CurrentHealth 0.0)
    (CallFunction|Dead)))

(fn Dead)

(fn O2Tick
  (if (> (Variables|Default|GetCurrentO2) 0.0)
    (bind _output_get (Variables|Default|SetCurrentO2 (- (Variables|Default|GetCurrentO2) 1.0)))
    (CallFunction|SetStatPercentage (Variables|/Game/UI/WB_PlayerStats.WB_PlayerStats_C|GetPB_Hunger (Variables|Default|GetWB%20Player%20Stats)) _output_get (Variables|Default|GetMaxO2))
    (else
      (CallFunction|ReceiveDamage 2.0))))

(fn SetStatPercentage
  (params (InputStat :type Progress%20Bar%20Object%20Reference) (Current :type Float%20%28double-precision%29) (Max :type Float%20%28double-precision%29))
  (Progress|SetPercent InputStat (/ Current Max)))

(fn GetLevelEXP
  (params (Skill :type E_Skills%20Enum :default "NewEnumerator0") (Level :type Integer))
  (bind _returnvalue (Utilities|GetDataTableRow "/Game/UI/DT_LevelExp.DT_LevelExp" (Utilities|String|StringToName (Utilities|String|EnumtoString Skill)))
    (:then
      (return (Utilities|Array|Get(acopy) (.NextLevelEXP (Utilities|Struct|BreakF_LevelExp _returnvalue)) Level)))))

(fn AddExptoSkill
  (params (Skill :type E_Skills%20Enum :default "NewEnumerator0") (ExpToAdd :type Float%20%28double-precision%29))
  (for (_array_element _array_index) (Variables|Default|GetSkills)
    (if (Utilities|Enum|Equal(Enum) (.Skill (Utilities|Struct|BreakF_LevelExp _array_element)) Skill)
      (Utilities|Array|SetArrayElem (Variables|Default|GetSkills) _array_index (Utilities|Struct|MakeF_LevelExp (.Skill (Utilities|Struct|BreakF_LevelExp (Utilities|Array|Get(acopy) (Variables|Default|GetSkills) _array_index))) (.Level (Utilities|Struct|BreakF_LevelExp (Utilities|Array|Get(acopy) (Variables|Default|GetSkills) _array_index))) (.NextLevelEXP (Utilities|Struct|BreakF_LevelExp (Utilities|Array|Get(acopy) (Variables|Default|GetSkills) _array_index))) (+ (.CurrentEXP (Utilities|Struct|BreakF_LevelExp (Utilities|Array|Get(acopy) (Variables|Default|GetSkills) _array_index))) ExpToAdd) (.Description (Utilities|Struct|BreakF_LevelExp (Utilities|Array|Get(acopy) (Variables|Default|GetSkills) _array_index))) (.SkillTexture (Utilities|Struct|BreakF_LevelExp (Utilities|Array|Get(acopy) (Variables|Default|GetSkills) _array_index)))))
      (return (.Skill (Utilities|Struct|BreakF_LevelExp (Utilities|Array|Get(acopy) (Variables|Default|GetSkills) _array_index))) (.Level (Utilities|Struct|BreakF_LevelExp (Utilities|Array|Get(acopy) (Variables|Default|GetSkills) _array_index))) (+ (.CurrentEXP (Utilities|Struct|BreakF_LevelExp (Utilities|Array|Get(acopy) (Variables|Default|GetSkills) _array_index))) ExpToAdd) _array_index))))

(fn CheckLevelUp
  (params (NextLevelExp :type Float%20%28double-precision%29) (CurrentExp :type Float%20%28double-precision%29) (CurrentLevel :type Integer) (SkillIndex :type Integer))
  (bind _skills (Variables|Default|GetSkills))
  (bind _output (Utilities|Array|Get(acopy) _skills SkillIndex))
  (bind (_skill _level _nextlevelexp _currentexp _description _skilltexture) (Utilities|Struct|BreakF_LevelExp _output))
  (if (< CurrentLevel 10)
    (if (<= NextLevelExp CurrentExp)
      (bind _result (Math|Integer|IncrementInt _level)
        (:%20%20
          (Utilities|Array|SetArrayElem (Variables|Default|GetSkills) SkillIndex (Utilities|Struct|MakeF_LevelExp _skill _result _nextlevelexp _currentexp _description _skilltexture))
          (return true)))
      (else
        (return false)))
    (else
      (return false))))

(fn AddExp
  (params (Skill :type E_Skills%20Enum :default "NewEnumerator0") (ExpToAdd :type Float%20%28double-precision%29))
  (bind (_currentskill _currentlevel _currentexp _skillindex) (CallFunction|AddExptoSkill Skill ExpToAdd))
  (bind _nextlevelexp (CallFunction|GetLevelEXP _currentskill _currentlevel))
  (bind _levelledup (CallFunction|CheckLevelUp _nextlevelexp _currentexp _currentlevel _skillindex))
  (if (and _levelledup (< _currentlevel 10))
    (bind _levelledup_2 (CallFunction|AddExp Skill 0.0))
    (return _levelledup_2)
    (else
      (return false))))

(fn RemoveO2Amount
  (params (O2Amount :type Float%20%28double-precision%29))
  (bind _output_get (Variables|Default|SetCurrentO2 (- (Variables|Default|GetCurrentO2) O2Amount)))
  (CallFunction|SetStatPercentage (Variables|/Game/UI/WB_PlayerStats.WB_PlayerStats_C|GetPB_Hunger (Variables|Default|GetWB%20Player%20Stats)) _output_get (Variables|Default|GetMaxO2))
  (return))

(fn AddMoveModifier
  (params (EffectValue :type Float%20%28double-precision%29) (MathType :type E_MathTypes%20Enum :default "NewEnumerator0"))
  (Utilities|Map|Add (Variables|Default|GetMoveSpeedMultiplier) EffectValue MathType)
  (CallFunction|CalculateMoveSpeed))

(fn CalculateMoveSpeed
  (Variables|Default|SetCurrentMoveSpeed (Variables|Default|GetBaseMoveSpeed))
  (bind _values (Utilities|Map|Values (Variables|Default|GetMoveSpeedMultiplier)))
  (for (_array_element _array_index) _values
    (if (Utilities|Enum|Equal(Enum) _array_element "NewEnumerator0")
      (bind _keys (Utilities|Map|Keys (Variables|Default|GetMoveSpeedMultiplier)))
      (Variables|Default|SetCurrentMoveSpeed (+ (Variables|Default|GetCurrentMoveSpeed) (Utilities|Array|Get(acopy) _keys _array_index)))))
  (bind _values_2 (Utilities|Map|Values (Variables|Default|GetMoveSpeedMultiplier)))
  (for (_array_element_2 _array_index_2) _values_2
    (if (Utilities|Enum|Equal(Enum) _array_element_2 "NewEnumerator1")
      (bind _keys_2 (Utilities|Map|Keys (Variables|Default|GetMoveSpeedMultiplier)))
      (Variables|Default|SetCurrentMoveSpeed (* (Variables|Default|GetCurrentMoveSpeed) (Utilities|Array|Get(acopy) _keys_2 _array_index_2)))))
  (Variables|/Script/Engine.CharacterMovementComponent|SetMaxWalkSpeed (Variables|/Script/Engine.Character|GetCharacterMovement (Variables|Default|GetAs%20BP%20First%20Person%20Character)) (Variables|Default|GetCurrentMoveSpeed)))

(fn RemoveMoveModifier
  (params (EffectValue :type Float%20%28double-precision%29) (MathType :type E_MathTypes%20Enum :default "NewEnumerator0"))
  (bind _keys (Utilities|Map|Keys (Variables|Default|GetMoveSpeedMultiplier)))
  (for (_array_element _array_index) _keys
    (if (== _array_element EffectValue)
      (bind _values (Utilities|Map|Values (Variables|Default|GetMoveSpeedMultiplier)))
      (if (Utilities|Enum|Equal(Enum) (Utilities|Array|Get(acopy) _values _array_index) MathType)
        (Utilities|Map|Remove (Variables|Default|GetMoveSpeedMultiplier) EffectValue)
        (CallFunction|CalculateMoveSpeed)
        (return))))
  (return))