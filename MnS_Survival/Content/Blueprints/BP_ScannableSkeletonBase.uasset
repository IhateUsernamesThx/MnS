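; Base Blueprint for skeletal-mesh objects that can be scanned and interacted with, exposing scan data, mesh and scanned state.
; Interacting spawns each Effect class as an actor owned by this object, passing effect strength, duration, skill, experience, harvest animation and item data built from the scan data.
; The construction script copies the data's Name into CustomName, and an event sets the Scanned flag.
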(event EventDoInteract
  (bind _data (Variables|AssetData|GetData))
  (bind (_name _customname _description) (Utilities|Struct|BreakF_ScannableData _data))
  (for _array_element (Variables|EffectStats|GetEffect)
    (Game|SpawnActorfromClass _array_element (Math|Transform|MakeTransform "0, 0, 0") "Undefined" "MultiplyWithRoot" self (Variables|EffectStats|GetEffect%20Magnitude) (Variables|EffectStats|GetEffect%20Duration) (Variables|EffectStats|GetSkill) (Variables|EffectStats|GetExp%20Amount) (Variables|AssetData|GetItem%20Name) (Utilities|Struct|MakeBP_ItemCustomData _name (Utilities|Struct|MakeFItemStruct "" "" (Variables|AssetData|GetThumbnail) 0 0 0 0 (Variables|AssetData|GetItem%20Type)) _customname _description (Variables|EffectStats|GetEffect)) (Variables|AssetData|GetHarvest%20Animation) 0)))

(event EventSetScanData
  (params (Scanned :type Boolean))
  (Variables|AssetData|SetScanned Scanned))

(fn ConstructionScript
  (bind _data (Variables|AssetData|GetData))
  (Utilities|Struct|SetmembersinF_ScannableData _data (.Name (Utilities|Struct|BreakF_ScannableData _data))))

(fn ReturnScanData
  (return (Variables|AssetData|GetData) (Variables|Default|GetSkeletalMesh) (Variables|AssetData|GetScanned)))