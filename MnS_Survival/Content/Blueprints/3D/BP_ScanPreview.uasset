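; Preview actor that renders a scanned object's static or skeletal mesh in isolation for display through a material.
; BeginPlay copies the referenced mesh asset and restricts a scene capture to it, targeting a small runtime render target.
; That target feeds a dynamic display material, exposed through ReturnObjectRT.
; The construction script applies a scan material to the static mesh's slots; the rotating-capture timeline is never triggered.
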(event EventBeginPlay
  (bind _meshref (Variables|Default|GetMeshRef))
  (bind _skeletalmesh (Variables|Default|GetSkeletalMesh))
  (bind _mesh (Variables|Default|GetMesh))
  (bind _asstatic_mesh_component (Utilities|Casting|CastToStaticMeshComponent _meshref)
    (:then
      (Components|StaticMesh|SetStaticMesh _mesh (Variables|/Script/Engine.StaticMeshComponent|GetStaticMesh _asstatic_mesh_component))
      (Rendering|SceneCapture|ShowOnlyComponent (Variables|Default|GetScanObject) _mesh))
    (:CastFailed
      (bind _asskeletal_mesh_component (Utilities|Casting|CastToSkeletalMeshComponent _meshref))
      (Components|SkeletalMesh|SetSkeletalMeshAsset _skeletalmesh (Variables|/Script/Engine.SkeletalMeshComponent|GetSkeletalMeshAsset _asskeletal_mesh_component))
      (Rendering|SceneCapture|ShowOnlyComponent (Variables|Default|GetScanObject) _skeletalmesh)))
  (bind _returnvalue (Rendering|CreateRenderTarget2D 160 160 "RTF_RGBA16f"))
  (bind _output_get (Variables|/Script/Engine.SceneCaptureComponent2D|SetTextureTarget (Variables|Default|GetScanObject) _returnvalue))
  (bind _returnvalue_2 (Rendering|Material|CreateDynamicMaterialInstance "/Game/Blueprints/3D/M_ScanObjectDisplay.M_ScanObjectDisplay" "None" "None" :!class /Script/Engine.KismetMaterialLibrary))
  (bind _output_get_2 (Variables|Default|SetObjectMaterial _returnvalue_2))
  (Rendering|Material|SetTextureParameterValue _output_get_2 "ScanTexture" _output_get))

(fn ConstructionScript
  (bind _mesh (Variables|Default|GetMesh))
  (for _index (range 0 (Rendering|Material|GetNumMaterials _mesh))
    (Rendering|Material|SetMaterial _mesh _index "/Game/Blueprints/3D/M_ScannedObject.M_ScannedObject")))

(fn ReturnObjectRT
  (return 0 (Variables|Default|GetObjectMaterial)))