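; BP_TerminalUplink is an interactable terminal actor that opens an uplink UI for the player.
; On BeginPlay it creates a WB_TerminalUplink widget, passes it the static mesh's world location and caches it.
; DoInteract adds that widget to the viewport, shows the mouse cursor, switches input to UI only and uses cinematic mode to lock movement and turning.
; The actor itself has no logic for closing the widget or restoring input.
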(event EventBeginPlay
  (bind _returnvalue (UserInterface|CreateWidget "/Game/UI/WB_TerminalUplink.WB_TerminalUplink_C" 0 (Transformation|GetWorldLocation (Variables|Default|GetStaticMesh))))
  (Variables|Default|SetTerminalWidget _returnvalue)
  (|CallParentFunction))

(event Collision|EventActorBeginOverlap
  (params (OtherActor :type Actor%20Object%20Reference))
  (|CallParentFunction OtherActor) ; This node is disabled and will not be called.\nDrag off pins to build functionality.
)

(event EventTick
  (params (DeltaSeconds :type Float%20%28single-precision%29))
  (|CallParentFunction DeltaSeconds) ; This node is disabled and will not be called.\nDrag off pins to build functionality.
)

(event EventDoInteract
  (bind _returnvalue (Game|GetPlayerController 0))
  (UserInterface|Viewport|AddtoViewport (Variables|Default|GetTerminalWidget) 0)
  (Variables|/Script/Engine.PlayerController|SetbShowMouseCursor _returnvalue true)
  (Input|SetInputModeUIOnly _returnvalue 0 "DoNotLock" false)
  (Class|PlayerController|SetCinematicMode _returnvalue true false false true true))

(fn ConstructionScript
  (|CallParentFunction))