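; Inventory component that stores item slot data in an indexed Content array.
; Add writes an item at a given index after checking it against InventorySize, Remove overwrites that slot with an empty entry, and both then call RefreshInventory.
; FindItemIndex searches by matching a slot struct built from the item ID.
; RefreshInventory, Drop and GetQuantity are empty stubs.
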(fn AddtoInventory
  (params (ItemData :type F%20Slot%20Data%20Structure) (Index :type Integer))
  (if (<= Index (Variables|Default|GetInventorySize))
    (Utilities|Array|SetArrayElem (Variables|Default|GetContent) Index ItemData)
    (CallFunction|RefreshInventory)
    (return)
    (else
      (return))))

(fn RemovefromInventory
  (params (Index :type Integer))
  (Utilities|Array|SetArrayElem :TargetArray (Variables|Default|GetContent) :Index Index)
  (CallFunction|RefreshInventory)
  (return))

(fn FindItemIndex
  (params (ItemID :type F%20Item%20Data%20Structure))
  (bind _id (Utilities|Struct|BreakF_ItemData ItemID))
  (bind _content (Variables|Default|GetContent))
  (bind _f_slotdata (Utilities|Struct|MakeF_SlotData _id))
  (bind _returnvalue (Utilities|Array|FindItem _content _f_slotdata))
  (if (> _returnvalue -1)
    (return _returnvalue)))

(fn Drop)

(fn RefreshInventory)

(fn GetQuantity
  (params (ItemID :type F%20Item%20Data%20Structure)))