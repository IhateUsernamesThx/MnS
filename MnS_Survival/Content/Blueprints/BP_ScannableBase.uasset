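; Base Blueprint for scannable items that track a scanned state and spawn effect actors when interacted with.
; Interaction loops over the Effect classes, spawning each at world origin with magnitude, duration, skill, experience and packed custom item data.
; ReturnScanData exposes the data, mesh and scanned flag, while SetScanData updates the flag.
; The construction script copies the data's Name into its CustomName.
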(event EventDoInteract
  (bind _data (Variables|Default|GetData))
  (bind (_name _customname _description) (Utilities|Struct|BreakF_ScannableData _data))
  (for _array_element (Variables|EffectStats|GetEffect)
    (Game|SpawnActorfromClass _array_element (Math|Transform|MakeTransform "0, 0, 0") "Undefined" "MultiplyWithRoot" 0 (Variables|EffectStats|GetEffect%20Magnitude) (Variables|EffectStats|GetEffect%20Duration) (Variables|EffectStats|GetSkill) (Variables|EffectStats|GetExp%20Amount) (Variables|Default|GetItem%20Name) (Utilities|Struct|MakeBP_ItemCustomData _name (Utilities|Struct|MakeFItemStruct "" "" (Variables|Default|GetThumbnail) 0 0 0 0 (Variables|Default|GetItem%20Type)) _customname _description (Variables|EffectStats|GetEffect)) 0)))

(event EventSetScanData
  (params (Scanned :type Boolean))
  (Variables|Default|SetScanned Scanned))

(fn ConstructionScript
  (bind _data (Variables|Default|GetData))
  (Utilities|Struct|SetmembersinF_ScannableData _data (.Name (Utilities|Struct|BreakF_ScannableData _data))))

(fn ReturnScanData
  (return (Variables|Default|GetData) (Variables|Default|GetStaticMesh) (Variables|Default|GetScanned)))