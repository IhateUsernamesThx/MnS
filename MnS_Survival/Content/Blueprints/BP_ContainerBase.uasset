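; BP_ContainerBase is a base Blueprint for interactable storage containers that open an inventory screen.
; On BeginPlay it creates a UI_ContainerInventory widget bound to its ContainerInventory component, labeled with the custom name from its Data, and caches the reference.
; DoInteract adds that cached widget to the viewport, while the construction script only calls its parent.
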(event EventDoInteract
  (UserInterface|Viewport|AddtoViewport (Variables|Default|GetContainerWidgetRef) 0))

(event EventBeginPlay
  (bind _returnvalue (UserInterface|CreateWidget "/Game/UI/Inventory/UI_ContainerInventory.UI_ContainerInventory_C" 0 (Variables|Default|GetContainerInventory) (Utilities|Text|ToText(Name) (Utilities|Struct|BreakF_ScannableData (Variables|Default|GetData))) "" 0))
  (Variables|Default|SetContainerWidgetRef _returnvalue))

(fn ConstructionScript
  (|CallParentFunction))