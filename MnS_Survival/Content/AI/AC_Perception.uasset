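; Creature perception component that tracks nearby perceivable actors by ecological role and turns threats into fear.
; UpdatePerception rebuilds KnownActors from a sphere overlap filtered by BPI_Perceivable, storing each actor's role and distance for closest-of-role queries.
; EvaluateStimuli matches known actors against the species' ThreatRoles, passing distance-based fear or the species' recovery rate to ACNeeds.
; It has no active Tick or BeginPlay, so setup and updates rely on external calls.
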(event EventBeginPlay)

(event EventTick
  (params (DeltaSeconds :type Float%20%28single-precision%29)))

(fn Initialise
  (params (CreatureOwner :type BP%20Creature%20Base%20Object%20Reference) (SpeciesData :type PDA%20Creature%20Species%20Object%20Reference))
  (bind _output_get (Variables|Default|SetCreatureOwner CreatureOwner))
  (Variables|Default|SetSpeciesData SpeciesData)
  (Variables|Default|SetAC%20Needs (Variables|/Game/AI/BP_CreatureBase.BP_CreatureBase_C|GetAC_Needs _output_get)))

(fn GetNearbyActors
  (params (Radius :type Float%20%28double-precision%29))
  (bind _outactors (Collision|SphereOverlapActors (Transformation|GetActorLocation (Components|GetOwner)) Radius (Utilities|Array|MakeArray "ObjectTypeQuery3" "ObjectTypeQuery2") 0 (Utilities|Array|MakeArray (Variables|Default|GetCreatureOwner))))
  (for _array_element _outactors
    (if (Utilities|DoesObjectImplementInterface _array_element "/Game/AI/BPI_Perceivable.BPI_Perceivable_C")
      (bind _perceptiontype (Class|BPIPerceivable|GetPerceptionType(Message) _array_element))
      (Utilities|Array|Add (LocalVariables|GetPerceivedActors) (Utilities|Struct|MakeF_PerceivedActor _array_element _perceptiontype (Math|Vector|Distance(Vector) (Transformation|GetActorLocation (Variables|Default|GetCreatureOwner)) (Transformation|GetActorLocation _array_element))))))
  (return (LocalVariables|GetPerceivedActors)))

(fn UpdatePerception
  (bind _actorarray (CallFunction|GetNearbyActors 2e+03))
  (Variables|Default|SetKnownActors _actorarray))

(fn GetClosestActorOfRole
  (params (EcologicalRole :type E_EcologicalRoles%20Enum :default "NewEnumerator0"))
  (for _array_element (Variables|Default|GetKnownActors)
    (if (== (.EcologicalRole (Utilities|Struct|BreakF_PerceivedActor _array_element)) EcologicalRole)
      (if (< (.Distance (Utilities|Struct|BreakF_PerceivedActor _array_element)) (LocalVariables|GetClosestDistance))
        (LocalVariables|SetClosestDistance (.Distance (Utilities|Struct|BreakF_PerceivedActor _array_element)))
        (LocalVariables|SetClosestPerceivedActor _array_element))))
  (return (< (LocalVariables|GetClosestDistance) 99999999.0) (LocalVariables|GetClosestPerceivedActor)))

(fn EvaluateStimuli
  (bind _speciesdata (Variables|Default|GetSpeciesData))
  (bind _threatroles (Variables|/Game/AI/PDA_CreatureSpecies.PDA_CreatureSpecies_C|GetThreatRoles _speciesdata))
  (if (not (Utilities|Array|IsEmpty _threatroles))
    (for _array_element _threatroles
      (for _array_element_2 (Variables|Default|GetKnownActors)
        (bind _perceptiontype (Class|BPIPerceivable|GetPerceptionType(Message) (.Actor (Utilities|Struct|BreakF_PerceivedActor _array_element_2))))
        (if (and (Utilities|Enum|Equal(Enum) _perceptiontype _array_element) (< (.Distance (Utilities|Struct|BreakF_PerceivedActor _array_element_2)) (LocalVariables|GetClosestThreatDistance)))
          (LocalVariables|SetClosestThreatDistance (.Distance (Utilities|Struct|BreakF_PerceivedActor _array_element_2)))
          (LocalVariables|SetDetectedThreat true)))
      (if (LocalVariables|GetDetectedThreat)
        (Default|ModifyFear (Variables|Default|GetAC%20Needs) (Math|Float|Clamp(Float) (- 1e+03 (LocalVariables|GetClosestThreatDistance)) 0.0 1e+02))
        (Development|PrintString (Utilities|String|ToString(Float) (Math|Float|Clamp(Float) (- 1e+03 (LocalVariables|GetClosestThreatDistance)) 0.0 1e+02)) true true "(R=1.000000,G=0.000000,B=0.017848,A=1.000000)")
        (else
          (Default|ModifyFear (Variables|Default|GetAC%20Needs) (Variables|/Game/AI/PDA_CreatureSpecies.PDA_CreatureSpecies_C|GetFearRecoveryRate (Variables|Default|GetSpeciesData))))))))