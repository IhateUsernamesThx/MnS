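; BP_CreatureBase is a base AI creature configured from its SpeciesData.
; The construction script applies the species mesh, animation Blueprint and walk speed.
; BeginPlay initialises movement, brain, needs and perception components, passing species data to all but movement.
; Each tick its widget rotates toward the player character, and GetPerceptionType reports the species' first role as its perception type.
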(event EventBeginPlay
  (bind _self self)
  (bind _speciesdata (Variables|Default|GetSpeciesData))
  (Default|Initialise (Variables|Default|GetAC_Movement) _self _self)
  (Default|InitialiseBrain (Variables|Default|GetAC_Brain) _speciesdata)
  (Default|Initialise (Variables|Default|GetAC_Needs) (Variables|/Game/AI/PDA_CreatureSpecies.PDA_CreatureSpecies_C|GetNeeds _speciesdata) (Variables|/Game/AI/PDA_CreatureSpecies.PDA_CreatureSpecies_C|GetNeedsRates _speciesdata))
  (Default|Initialise (Variables|Default|GetAC_Perception) self (Variables|Default|GetSpeciesData)))

(event EventTick
  (params (DeltaSeconds :type Float%20%28single-precision%29))
  (Transformation|SetWorldRotation (Variables|Default|GetWidget) (Math|Rotator|FindLookatRotation (Transformation|GetActorLocation) (Transformation|GetActorLocation (Game|GetPlayerCharacter 0))) false false))

(fn ConstructionScript
  (Components|SkeletalMesh|SetSkeletalMeshAsset (Variables|Character|GetMesh) (Variables|/Game/AI/PDA_CreatureSpecies.PDA_CreatureSpecies_C|GetSkeletalMesh (Variables|Default|GetSpeciesData)))
  (Class|SkeletalMeshComponent|SetAnimClass (Variables|Character|GetMesh) (Variables|/Game/AI/PDA_CreatureSpecies.PDA_CreatureSpecies_C|GetAnimBP (Variables|Default|GetSpeciesData)))
  (Variables|/Script/Engine.CharacterMovementComponent|SetMaxWalkSpeed (Variables|Character|GetCharacterMovement) (Variables|/Game/AI/PDA_CreatureSpecies.PDA_CreatureSpecies_C|GetMovementSpeed (Variables|Default|GetSpeciesData))))

(fn GetPerceptionType
  (return (Utilities|Array|Get(acopy) (Variables|/Game/AI/PDA_CreatureSpecies.PDA_CreatureSpecies_C|GetRoles (Variables|Default|GetSpeciesData)))))