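; AC_Brain is a creature AI component that picks and runs behaviours using utility scoring.
; It constructs behaviours from species data, injecting needs, movement and perception components, then re-scores them on a looping timer.
; A new best behaviour takes over only once the current one completes, updating the creature's AI state widget.
; Tick drives the active behaviour, while a separate timer refreshes perception and evaluates stimuli.
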(event Custom|EvaluationTick
  (bind _returnvalue (Components|GetOwner))
  (bind _returnvalue_2 (Actor|GetComponentbyClass _returnvalue "/Game/AI/AC_Perception.AC_Perception_C"))
  (Default|UpdatePerception _returnvalue_2)
  (Default|EvaluateStimuli _returnvalue_2))

(event EventBeginPlay
  (Utilities|Time|SetTimerbyEvent (delegate Custom|EvaluationTick) 0.5 true))

(event EventTick
  (params (DeltaSeconds :type Float%20%28single-precision%29))
  (bind _currentbehaviour (Variables|Default|GetCurrentBehaviour)
    (:then
      (Default|TickBehaviour _currentbehaviour DeltaSeconds))
    (:else)))

(fn InitialiseBehaviours
  (for _array_element (Variables|/Game/AI/PDA_CreatureSpecies.PDA_CreatureSpecies_C|GetBehaviourClasses (Variables|Default|GetSpeciesData))
    (bind _returnvalue (Game|ConstructObjectfromClass _array_element))
    (bind _asbp_behaviour_base (Utilities|Casting|CastToBP_BehaviourBase _returnvalue))
    (bind _ascharacter (Utilities|Casting|CastToCharacter (Components|GetOwner)))
    (Default|Initialise _asbp_behaviour_base self _ascharacter (Variables|Default|GetSpeciesData) (Actor|GetComponentbyClass _ascharacter "/Game/AI/AC_Needs.AC_Needs_C") (Actor|GetComponentbyClass (Components|GetOwner) "/Game/AI/AC_Movement.AC_Movement_C") (Actor|GetComponentbyClass (Components|GetOwner) "/Game/AI/AC_Perception.AC_Perception_C"))
    (Utilities|Array|Add (Variables|Default|GetBehaviourList) _asbp_behaviour_base))
  (CallFunction|EvaluateBehaviours))

(fn InitialiseBrain
  (params (SpeciesData :type PDA%20Creature%20Species%20Object%20Reference))
  (Variables|Default|SetSpeciesData SpeciesData)
  (CallFunction|InitialiseBehaviours)
  (Utilities|Time|SetTimerbyFunctionName 0 "EvaluateBehaviours" 0.2 true))

(fn EvaluateBehaviours
  (for _array_element (Variables|Default|GetBehaviourList)
    (bind _score (Default|Evaluate _array_element))
    (if (> _score (LocalVariables|GetBestScore))
      (LocalVariables|SetBestScore _score)
      (LocalVariables|SetBestBehaviour _array_element)))
  (if (!= (LocalVariables|GetBestBehaviour) (Variables|Default|GetCurrentBehaviour))
    (if (!= (Variables|Default|GetCurrentBehaviour) 0)
      (bind _finished (Default|IsComplete (Variables|Default|GetCurrentBehaviour)))
      (if _finished
        (Variables|/Game/AI/BP_BehaviourBase.BP_BehaviourBase_C|SetIsActive (Variables|Default|GetCurrentBehaviour) false)
        (Default|Exit (Variables|Default|GetCurrentBehaviour))
        (Variables|Default|SetPreviousBehaviour (Variables|Default|GetCurrentBehaviour))
        (bind _output_get (Variables|Default|SetCurrentBehaviour (LocalVariables|GetBestBehaviour)))
        (Variables|/Game/AI/BP_BehaviourBase.BP_BehaviourBase_C|SetIsActive _output_get true)
        (Default|Enter _output_get)
        (bind _asbp_creature_base (Utilities|Casting|CastToBP_CreatureBase (Components|GetOwner) :!label _label))
        (bind _aswbp_aistate (Utilities|Casting|CastToWBP_AIState (UserInterface|GetWidget (Variables|/Game/AI/BP_CreatureBase.BP_CreatureBase_C|GetWidget _asbp_creature_base))))
        (Default|UpdateState _aswbp_aistate (Utilities|Text|ToText(String) (Utilities|GetDisplayName (Variables|Default|GetCurrentBehaviour)))))
      (else
        (bind _output_get_2 (Variables|Default|SetCurrentBehaviour (LocalVariables|GetBestBehaviour)))
        (Variables|/Game/AI/BP_BehaviourBase.BP_BehaviourBase_C|SetIsActive _output_get_2 true)
        (Default|Enter _output_get_2)
        (goto _label)))))