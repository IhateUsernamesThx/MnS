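; Creature movement component that turns travel requests into move requests on the owner's BP_CreatureAIController.
; It can travel to a random navmesh-projected point, a location or an actor, move directly away from a threat, or stop.
; Each travel call sets movement flags and a state, while HasReachedDestination resets them and fires OnDestinationReached.
; TravelToActor completes immediately when the target is already within range.
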(event EventTick
  (params (DeltaSeconds :type Float%20%28single-precision%29)))

(fn Initialise
  (params (CreatureOwner :type BP%20Creature%20Base%20Object%20Reference) (CharacterOwner :type Character%20Object%20Reference))
  (Variables|Default|SetCreatureOwner CreatureOwner)
  (Variables|Default|SetCharacterOwner CharacterOwner))

(fn TraveltoRandom
  (bind _creatureowner (Variables|Default|GetCreatureOwner))
  (Variables|Default|SetMoving true)
  (Variables|Default|SetMoveCompleted false)
  (Development|PrintString (Utilities|GetDisplayName _creatureowner))
  (bind (_location _success) (CallFunction|GetRandomReachableLocation (Transformation|GetActorLocation _creatureowner) 2.5e+02 1e+03))
  (if _success
    (bind _asbp_creature_aicontroller (Utilities|Casting|CastToBP_CreatureAIController (AI|GetAIController _creatureowner)))
    (Default|RequestMove _asbp_creature_aicontroller _location 2e+01)
    (Variables|Default|SetState "NewEnumerator1")))

(fn TraveltoLocation
  (params (TargetLocation :type Vector))
  (Variables|Default|SetMoving true)
  (Variables|Default|SetMoveCompleted false)
  (bind _asbp_creature_aicontroller (Utilities|Casting|CastToBP_CreatureAIController (AI|GetAIController (Variables|Default|GetCreatureOwner))))
  (Default|RequestMove _asbp_creature_aicontroller TargetLocation 1.5e+02)
  (Variables|Default|SetState "NewEnumerator1"))

(fn TraveltoActor
  (params (TargetActor :type Actor%20Object%20Reference))
  (bind _returnvalue (Transformation|GetActorLocation TargetActor))
  (bind _creatureowner (Variables|Default|GetCreatureOwner))
  (Variables|Default|SetMoving true)
  (Variables|Default|SetMoveCompleted false)
  (if (< (Math|Vector|Distance(Vector) (Transformation|GetActorLocation _creatureowner) _returnvalue) 1.5e+02)
    (CallFunction|HasReachedDestination (Variables|/Game/AI/BP_CreatureBase.BP_CreatureBase_C|GetAC_Movement (Variables|Default|GetCreatureOwner)))
    (else
      (bind _asbp_creature_aicontroller (Utilities|Casting|CastToBP_CreatureAIController (AI|GetAIController _creatureowner)))
      (Default|RequestMove _asbp_creature_aicontroller _returnvalue 1.5e+02)
      (Variables|Default|SetState "NewEnumerator1"))))

(fn TravelAwayfrom
  (params (ThreatActor :type Actor%20Object%20Reference) (Distance :type Float%20%28double-precision%29))
  (bind _returnvalue (Components|GetOwner))
  (bind _returnvalue_2 (Transformation|GetActorLocation ThreatActor))
  (bind _returnvalue_3 (Transformation|GetActorLocation _returnvalue))
  (bind _returnvalue_4 (- _returnvalue_3 _returnvalue_2))
  (bind _returnvalue_5 (Math|Vector|Normalize _returnvalue_4))
  (bind _returnvalue_6 (* _returnvalue_5 Distance))
  (Variables|Default|SetMoving true)
  (Variables|Default|SetMoveCompleted false)
  (bind _asbp_creature_aicontroller (Utilities|Casting|CastToBP_CreatureAIController (AI|GetAIController (Variables|Default|GetCreatureOwner))))
  (Default|RequestMove _asbp_creature_aicontroller (+ _returnvalue_3 _returnvalue_6) 1.5e+02)
  (Variables|Default|SetState "NewEnumerator1")
  (Development|PrintString (Utilities|String|ToString(Text) (Utilities|Text|FormatText "{0} 
{1}" (Utilities|String|ToString(Vector) _returnvalue_3) (Utilities|String|ToString(Vector) _returnvalue_6))) true true "(R=0.000000,G=1.000000,B=0.142942,A=1.000000)" 2e+01))

(fn Stop
  (bind _asbp_creature_aicontroller (Utilities|Casting|CastToBP_CreatureAIController (AI|GetAIController (Variables|Default|GetCreatureOwner))))
  (Default|StopMove _asbp_creature_aicontroller))

(fn IsMoving
  (return (Variables|Default|GetState)))

(fn CheckDestinationReached
  (return "Success" (Variables|Default|GetMoveCompleted)))

(fn GetRandomReachableLocation
  (params (Origin :type Vector) (MinDistance :type Float%20%28double-precision%29) (MaxDistance :type Float%20%28double-precision%29))
  (bind _returnvalue (Math|Random|RandomFloatinRange MinDistance MaxDistance))
  (bind _randomlocation (AI|Navigation|GetRandomReachablePointinRadius Origin _returnvalue 0 0))
  (bind (_projectedlocation _returnvalue_2) (AI|Navigation|ProjectPointtoNavigation _randomlocation 0 0 "0, 0, 0"))
  (return _projectedlocation _returnvalue_2))

(fn HasReachedDestination
  (Variables|Default|SetMoveCompleted true)
  (Variables|Default|SetMoving false)
  (Variables|Default|SetState "NewEnumerator0")
  (Default|CallOnDestinationReached))