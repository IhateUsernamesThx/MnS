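; Actor component that tracks an AI creature's hunger, fatigue, curiosity and fear, seeded from species needs and metabolism rates.
; Getters expose each need, and Modify functions add to values clamped between fixed bounds.
; Tick prints a debug readout and applies passive change to hunger only.
; ModifyCuriosity writes its result into Hunger, so Curiosity never changes through it.
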(event EventTick
  (params (DeltaSeconds :type Float%20%28single-precision%29))
  (bind _currentneeds (Variables|Default|GetCurrentNeeds))
  (bind (_hunger _fatigue _curiosity _fear) (Utilities|Struct|BreakF_BaseNeeds _currentneeds))
  (Development|PrintString (Utilities|String|ToString(Text) (Utilities|Text|FormatText "{4} 
Hunger: {0} 
Fatigue: {1} 
Curiosity: {2} 
Fear: {3}" _hunger _fatigue _curiosity _fear (Utilities|GetDisplayName (Components|GetOwner)))) true true "(R=0.000000,G=0.660000,B=1.000000,A=1.000000)" 0.001)
  (CallFunction|PassiveUpdates DeltaSeconds))

(fn Initialise
  (params (SpeciesNeeds :type F%20Base%20Needs%20Structure) (MetabolismRates :type F%20Behaviour%20Rates%20Structure))
  (Variables|Default|SetCurrentNeeds SpeciesNeeds)
  (Variables|Default|SetMetabolismRates MetabolismRates))

(fn GetHunger
  (return (Utilities|Struct|BreakF_BaseNeeds (Variables|Default|GetCurrentNeeds))))

(fn GetFear
  (return (Utilities|Struct|BreakF_BaseNeeds (Variables|Default|GetCurrentNeeds))))

(fn GetFatigue
  (return (Utilities|Struct|BreakF_BaseNeeds (Variables|Default|GetCurrentNeeds))))

(fn GetCuriosity
  (return (Utilities|Struct|BreakF_BaseNeeds (Variables|Default|GetCurrentNeeds))))

(fn ModifyHunger
  (params (AddedValue :type Float%20%28double-precision%29))
  (bind _structout (Utilities|Struct|SetmembersinF_BaseNeeds (Variables|Default|GetCurrentNeeds) (Math|Float|Clamp(Float) (+ AddedValue (Utilities|Struct|BreakF_BaseNeeds (Variables|Default|GetCurrentNeeds))) 0.0 1e+02)))
  (Variables|Default|SetCurrentNeeds _structout))

(fn ModifyFear
  (params (AddedValue :type Float%20%28double-precision%29))
  (bind _structout (Utilities|Struct|SetmembersinF_BaseNeeds (Variables|Default|GetCurrentNeeds) (Math|Float|Clamp(Float) (+ AddedValue (Utilities|Struct|BreakF_BaseNeeds (Variables|Default|GetCurrentNeeds))) 0.0 1e+02)))
  (Variables|Default|SetCurrentNeeds _structout))

(fn ModifyFatigue
  (params (AddedValue :type Float%20%28double-precision%29))
  (bind _structout (Utilities|Struct|SetmembersinF_BaseNeeds (Variables|Default|GetCurrentNeeds) (Math|Float|Clamp(Float) (+ AddedValue (Utilities|Struct|BreakF_BaseNeeds (Variables|Default|GetCurrentNeeds))) 0.0 1e+02)))
  (Variables|Default|SetCurrentNeeds _structout))

(fn ModifyCuriosity
  (params (AddedValue :type Float%20%28double-precision%29))
  (bind _structout (Utilities|Struct|SetmembersinF_BaseNeeds (Variables|Default|GetCurrentNeeds) (Math|Float|Clamp(Float) (+ AddedValue (Utilities|Struct|BreakF_BaseNeeds (Variables|Default|GetCurrentNeeds))) 0.0 1e+02)))
  (Variables|Default|SetCurrentNeeds _structout))

(fn PassiveUpdates
  (params (DeltaTime :type Float%20%28double-precision%29))
  (CallFunction|ModifyHunger (* DeltaTime (Utilities|Struct|BreakF_BehaviourRates (Variables|Default|GetMetabolismRates)))))