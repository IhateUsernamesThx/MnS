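; BP_BehaviourBase is the base Blueprint for creature AI behaviours.
; Initialise caches the brain, owning creature, species data, Needs, Movement and Perception, and takes the behaviour's rates from the species' NeedsRates.
; It exposes Evaluate, CanExecute, Enter, TickBehaviour, Exit and IsComplete as stub hooks, with Evaluate returning zero and IsComplete returning true by default.
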(fn Initialise
  (params (InBrain :type AC%20Brain%20Object%20Reference) (InOwnerCreature :type Character%20Object%20Reference) (InSpeciesData :type PDA%20Creature%20Species%20Object%20Reference) (Needs :type AC%20Needs%20Object%20Reference) (Movement :type AC%20Movement%20Object%20Reference) (Perception :type AC%20Perception%20Object%20Reference))
  (Variables|Default|SetBrainRef InBrain)
  (Variables|Default|SetOwnerCreature InOwnerCreature)
  (Variables|Default|SetSpeciesData InSpeciesData)
  (Variables|Default|SetNeeds Needs)
  (Variables|Default|SetBehaviourRates (Variables|/Game/AI/PDA_CreatureSpecies.PDA_CreatureSpecies_C|GetNeedsRates (Variables|Default|GetSpeciesData)))
  (Variables|Default|SetMovement Movement)
  (Variables|Default|SetPerception Perception))

(fn Evaluate
  (return 0.0))

(fn Enter)

(fn Exit)

(fn TickBehaviour
  (params (DeltaTime :type Float%20%28double-precision%29)))

(fn CanExecute)

(fn IsComplete
  (return true))