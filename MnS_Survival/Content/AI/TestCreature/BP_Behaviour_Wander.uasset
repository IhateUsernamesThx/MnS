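; Wander behaviour for the test creature AI, sending it to random destinations with pauses in between.
; Evaluate returns a constant score, and Enter starts the first random trip through the Movement component.
; TickBehaviour applies wander fatigue to Needs and alternates between travelling and waiting for a random time within species pause limits.
; Exit stops movement, as does IsComplete before returning the parent's result.
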(fn Initialise
  (params (InBrain :type AC%20Brain%20Object%20Reference) (InOwnerCreature :type Character%20Object%20Reference) (InSpeciesData :type PDA%20Creature%20Species%20Object%20Reference) (Needs :type AC%20Needs%20Object%20Reference) (Movement :type AC%20Movement%20Object%20Reference) (Perception :type AC%20Perception%20Object%20Reference))
  (Development|PrintString 0 "Test Creature Initialised")
  (|CallParentFunction InBrain InOwnerCreature InSpeciesData Needs Movement Perception))

(fn Evaluate
  (return 3e+01))

(fn Enter
  (Default|TraveltoRandom (Variables|Default|GetMovement))
  (Variables|Default|SetWanderState "NewEnumerator1")
  (|CallParentFunction))

(fn Exit
  (Default|Stop (Variables|Default|GetMovement))
  (|CallParentFunction))

(fn TickBehaviour
  (params (DeltaTime :type Float%20%28double-precision%29))
  (Default|ModifyFatigue (Variables|Default|GetNeeds) (* (Utilities|Struct|BreakF_BehaviourRates (Variables|Default|GetBehaviourRates)) DeltaTime))
  (|CallParentFunction 0.0)
  (if (Utilities|Enum|Equal(Enum) (Variables|Default|GetWanderState) "NewEnumerator1")
    (if (.Success (Default|CheckDestinationReached (Variables|Default|GetMovement)))
      (CallFunction|StartWaiting))
    (elif (Utilities|Enum|Equal(Enum) (Variables|Default|GetWanderState) "NewEnumerator2")
      (bind _output_get (Variables|Default|SetWaitTimer (- (Variables|Default|GetWaitTimer) DeltaTime)))
      (if (<= _output_get 0.0)
        (Default|TraveltoRandom (Variables|Default|GetMovement))
        (Variables|Default|SetWanderState "NewEnumerator1")))))

(fn IsComplete
  (Default|Stop (Variables|Default|GetMovement))
  (bind _finished (|CallParentFunction))
  (return _finished))

(fn StartWaiting
  (bind _speciesdata (Variables|Default|GetSpeciesData))
  (Variables|Default|SetWaitTimer (Math|Random|RandomFloatinRange (Variables|/Game/AI/PDA_CreatureSpecies.PDA_CreatureSpecies_C|GetPauseMin _speciesdata) (Variables|/Game/AI/PDA_CreatureSpecies.PDA_CreatureSpecies_C|GetPauseMax _speciesdata)))
  (Variables|Default|SetWanderState "NewEnumerator2"))