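; BP_Behaviour_Idle is the idle behaviour for the test creature's AI, apparently a placeholder.
; Evaluate always returns a constant score, independent of needs or state.
; Initialise, Enter and Exit print debug strings and call their parent versions, though Initialise does not forward Movement.
; TickBehaviour only calls the parent, passing zero instead of DeltaTime.
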(fn Initialise
  (params (InBrain :type AC%20Brain%20Object%20Reference) (InOwnerCreature :type Character%20Object%20Reference) (InSpeciesData :type PDA%20Creature%20Species%20Object%20Reference) (Needs :type AC%20Needs%20Object%20Reference) (Movement :type AC%20Movement%20Object%20Reference))
  (Development|PrintString 0 "Test Creature Initialised")
  (|CallParentFunction InBrain InOwnerCreature InSpeciesData Needs 0))

(fn Evaluate
  (return 1e+01))

(fn Enter
  (Development|PrintString 0 "Entering Idle")
  (|CallParentFunction))

(fn Exit
  (Development|PrintString 0 "Exiting Idle")
  (|CallParentFunction))

(fn TickBehaviour
  (params (DeltaTime :type Float%20%28double-precision%29))
  (|CallParentFunction 0.0))