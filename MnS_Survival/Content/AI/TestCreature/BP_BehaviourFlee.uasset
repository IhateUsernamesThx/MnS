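; Flee behaviour for the test creature AI, scored by the creature's Fear need.
; On entry it stops current movement, switches to sprint speed and travels away from the closest perceived actor of a given role, exiting if none is found.
; Each time it reaches its destination while fear stays high, it flees again from that same stored threat.
; It completes when fear falls to the threshold.
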(fn Initialise
  (params (InBrain :type AC%20Brain%20Object%20Reference) (InOwnerCreature :type Character%20Object%20Reference) (InSpeciesData :type PDA%20Creature%20Species%20Object%20Reference) (Needs :type AC%20Needs%20Object%20Reference) (Movement :type AC%20Movement%20Object%20Reference) (Perception :type AC%20Perception%20Object%20Reference))
  (Development|PrintString 0 "Test Creature Initialised")
  (|CallParentFunction InBrain InOwnerCreature InSpeciesData Needs Movement Perception))

(fn Evaluate
  (return (Default|GetFear (Variables|Default|GetNeeds))))

(fn Enter
  (bind _ownercreature (Variables|Default|GetOwnerCreature))
  (bind _charactermovement (Variables|/Script/Engine.Character|GetCharacterMovement _ownercreature))
  (EventDispatchers|UnbindallEventsfromOnDestinationReached (Variables|Default|GetMovement))
  (Components|Movement|StopMovementImmediately _charactermovement)
  (Variables|/Script/Engine.CharacterMovementComponent|SetMaxWalkSpeed _charactermovement (Variables|/Game/AI/PDA_CreatureSpecies.PDA_CreatureSpecies_C|GetSprintSpeed (Variables|Default|GetSpeciesData)))
  (bind (_success _perceivedactor) (Default|GetClosestActorOfRole (Variables|Default|GetPerception) "NewEnumerator1"))
  (if _success
    (Variables|Default|SetThreatActor _perceivedactor)
    (Default|TravelAwayfrom (Variables|Default|GetMovement) (.Actor (Utilities|Struct|BreakF_PerceivedActor _perceivedactor)) (Variables|/Game/AI/PDA_CreatureSpecies.PDA_CreatureSpecies_C|GetFleeDistance (Variables|Default|GetSpeciesData)))
    (else
      (CallFunction|Exit))))

(fn Exit
  (|CallParentFunction))

(fn TickBehaviour
  (params (DeltaTime :type Float%20%28double-precision%29))
  (if (.Success (Default|CheckDestinationReached (Variables|Default|GetMovement)))
    (if (> (Default|GetFear (Variables|Default|GetNeeds)) 5.0)
      (Default|TravelAwayfrom (Variables|Default|GetMovement) (.Actor (Utilities|Struct|BreakF_PerceivedActor (Variables|Default|GetThreatActor))) (Variables|/Game/AI/PDA_CreatureSpecies.PDA_CreatureSpecies_C|GetFleeDistance (Variables|Default|GetSpeciesData))))))

(fn IsComplete
  (return (<= (Default|GetFear (Variables|Default|GetNeeds)) (Variables|Default|GetFearThreshold))))