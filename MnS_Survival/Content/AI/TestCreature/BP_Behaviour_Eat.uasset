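; Creature AI behaviour for eating, scored by the current hunger need and complete once hunger falls to the fed threshold.
; On entry it finds the closest perceived actor of a set role, travelling to it unless already in range, or exits if none is found.
; On arrival it sends the food a consume message and switches to Consuming.
; Each tick modifies fatigue, and also hunger while consuming.
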(fn Initialise
  (params (InBrain :type AC%20Brain%20Object%20Reference) (InOwnerCreature :type Character%20Object%20Reference) (InSpeciesData :type PDA%20Creature%20Species%20Object%20Reference) (Needs :type AC%20Needs%20Object%20Reference) (Movement :type AC%20Movement%20Object%20Reference) (Perception :type AC%20Perception%20Object%20Reference))
  (Development|PrintString 0 "Test Creature Initialised")
  (|CallParentFunction InBrain InOwnerCreature InSpeciesData Needs Movement Perception))

(fn Evaluate
  (return (Default|GetHunger (Variables|Default|GetNeeds))))

(fn Enter
  (Default|Stop (Variables|Default|GetMovement))
  (bind (_success _perceivedactor) (Default|GetClosestActorOfRole (Variables|Default|GetPerception) "NewEnumerator0"))
  (if _success
    (Variables|Default|SetTargetFood _perceivedactor)
    (if (< (.Distance (Utilities|Struct|BreakF_PerceivedActor _perceivedactor)) 1.5e+02)
      ;[1 1 1] Skip AI MoveTo if already within range
      (CallFunction|OnArrivedatFood)
      (else
        (EventDispatchers|BindEventtoOnDestinationReached (Variables|Default|GetMovement) (EventDispatchers|CreateEvent :!event OnArrivedatFood))
        (Default|TraveltoLocation (Variables|Default|GetMovement) (Transformation|GetActorLocation (.Actor (Utilities|Struct|BreakF_PerceivedActor _perceivedactor))))
        (Variables|Default|SetEatState "NewEnumerator0")))
    (else
      (CallFunction|Exit))))

(fn Exit
  (|CallParentFunction))

(fn TickBehaviour
  (params (DeltaTime :type Float%20%28double-precision%29))
  (Default|ModifyFatigue (Variables|Default|GetNeeds) (* 1.0 DeltaTime))
  (switch Utilities|FlowControl|Switch|SwitchonE_EatState (Variables|Default|GetEatState)
    (:NewEnumerator1
      (Default|ModifyHunger (Variables|Default|GetNeeds) (* (Utilities|Struct|BreakF_BehaviourRates (Variables|Default|GetBehaviourRates)) DeltaTime)))))

(fn IsComplete
  (return (<= (Default|GetHunger (Variables|Default|GetNeeds)) (Variables|Default|GetFedThreshold))))

(fn OnArrivedatFood
  (Class|BPIConsumable|Consume(Message) (.Actor (Utilities|Struct|BreakF_PerceivedActor (Variables|Default|GetTargetFood))) (Variables|Default|GetOwnerCreature))
  (Variables|Default|SetEatState "NewEnumerator1")
  (EventDispatchers|UnbindallEventsfromOnDestinationReached (Variables|Default|GetMovement)))