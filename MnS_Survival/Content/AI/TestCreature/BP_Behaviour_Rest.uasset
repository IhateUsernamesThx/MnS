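; Rest behaviour for test creature AI, scored by the creature's current fatigue.
; On entry it stops movement, then each tick modifies fatigue through Needs at the rest recovery rate scaled by delta time.
; It reports complete once fatigue is at or below the rested threshold.
; The parent tick receives zero rather than delta time, and the parent initialise is not passed Perception.
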(fn Initialise
  (params (InBrain :type AC%20Brain%20Object%20Reference) (InOwnerCreature :type Character%20Object%20Reference) (InSpeciesData :type PDA%20Creature%20Species%20Object%20Reference) (Needs :type AC%20Needs%20Object%20Reference) (Movement :type AC%20Movement%20Object%20Reference) (Perception :type AC%20Perception%20Object%20Reference))
  (Development|PrintString 0 "Test Creature Initialised")
  (|CallParentFunction InBrain InOwnerCreature InSpeciesData Needs Movement 0))

(fn Evaluate
  (return (Default|GetFatigue (Variables|Default|GetNeeds))))

(fn Enter
  (Default|Stop (Variables|Default|GetMovement))
  (|CallParentFunction))

(fn Exit
  (|CallParentFunction))

(fn TickBehaviour
  (params (DeltaTime :type Float%20%28double-precision%29))
  (Default|ModifyFatigue (Variables|Default|GetNeeds) (* (Utilities|Struct|BreakF_BehaviourRates (Variables|Default|GetBehaviourRates)) DeltaTime))
  (|CallParentFunction 0.0))

(fn IsComplete
  (return (<= (Default|GetFatigue (Variables|Default|GetNeeds)) (Variables|Default|GetRestedThreshold))))