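; AI controller for creatures that carries out move requests on its controlled pawn.
; RequestMove runs AI MoveTo toward a given destination and acceptance radius, and StopMove halts movement.
; A handler bound to ReceiveMoveCompleted on BeginPlay calls HasReachedDestination on the BP_CreatureBase movement component, whatever the result, then prints that result.
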(event Custom|RequestMove
  (params (Destination :type Vector) (AcceptanceRadius :type Float%20%28double-precision%29))
  (AI|AIMoveTo (Pawn|GetControlledPawn) Destination 0 AcceptanceRadius false))

(event Custom|StopMove
  (AI|Navigation|StopMovement))

(event Custom|MoveCompleted
  (params (RequestID :type AI%20Request%20ID%20Structure) (Result :type EPathFollowingResult%20Enum :default "Success"))
  (bind _asbp_creature_base (Utilities|Casting|CastToBP_CreatureBase (Pawn|GetControlledPawn)))
  (Default|HasReachedDestination (Variables|/Game/AI/BP_CreatureBase.BP_CreatureBase_C|GetAC_Movement _asbp_creature_base))
  (Development|PrintString (Utilities|String|EnumtoString Result)))

(event EventBeginPlay
  (EventDispatchers|BindEventtoReceiveMoveCompleted (EventDispatchers|CreateEvent :!event Custom|MoveCompleted)))

(fn ConstructionScript)