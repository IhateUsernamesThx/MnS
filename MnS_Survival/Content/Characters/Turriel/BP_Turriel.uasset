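; BP_Turriel is the Turriel character, which smoothly turns its head toward a nearby player and can be scanned.
; A fast looping timer drives the head look, interpolating the anim blueprint's look alpha by distance and passing it the player's look location.
; Scan functions store the scanned flag and return its data and mesh.
; Observed and interact events are empty; terminal widget and blackboard logic is disconnected.
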(event Custom|HeadLookDetection
  (bind _as_abp_turriel (Variables|Default|GetAs%20ABP%20Turriel))
  ;[1 0.4233 0] Smooth Head Look
  (if (< (Transformation|GetDistanceTo (Variables|Default|GetPlayerRef)) 7e+02) ; Check player is in range
    (Variables|/Game/Characters/Turriel/Animations/ABP_Turriel.ABP_Turriel_C|SetHeadLookAlpha _as_abp_turriel (Math|Interpolation|FInterpTo (Variables|/Game/Characters/Turriel/Animations/ABP_Turriel.ABP_Turriel_C|GetHeadLookAlpha (Variables|Default|GetAs%20ABP%20Turriel)) 1.0 (Utilities|Time|GetWorldDeltaSeconds) 2.0))
    (Variables|/Game/Characters/Turriel/Animations/ABP_Turriel.ABP_Turriel_C|SetHeadLookLocation _as_abp_turriel (Transformation|GetWorldLocation (Variables|/Game/FirstPerson/Blueprints/BP_FirstPersonCharacter.BP_FirstPersonCharacter_C|GetHeadLookLoc (Variables|Default|GetPlayerRef))))
    (elif (> (Variables|/Game/Characters/Turriel/Animations/ABP_Turriel.ABP_Turriel_C|GetHeadLookAlpha (Variables|Default|GetAs%20ABP%20Turriel)) 0.0) ; Check value is above 0 to prevent constant code firing
      (Variables|/Game/Characters/Turriel/Animations/ABP_Turriel.ABP_Turriel_C|SetHeadLookAlpha (Variables|Default|GetAs%20ABP%20Turriel) (Math|Interpolation|FInterpTo (Variables|/Game/Characters/Turriel/Animations/ABP_Turriel.ABP_Turriel_C|GetHeadLookAlpha (Variables|Default|GetAs%20ABP%20Turriel)) 0.0 (Utilities|Time|GetWorldDeltaSeconds) 2.0)))))

(event EventBeginPlay
  ;[0.1886 0.4336 1] Set initial variables
  (bind _asbp_first_person_character (Utilities|Casting|CastToBP_FirstPersonCharacter (Game|GetPlayerCharacter 0)))
  (Variables|Default|SetPlayerRef _asbp_first_person_character) ; Get player reference
  (bind _asabp_turriel (Utilities|Casting|CastToABP_Turriel (Components|SkeletalMesh|GetAnimInstance (Variables|Character|GetMesh))))
  (Variables|Default|SetAs%20ABP%20Turriel _asabp_turriel)
  (Utilities|Time|SetTimerbyEvent (EventDispatchers|CreateEvent :!event Custom|HeadLookDetection) 0.005 true) ; HeadLookTimer
)

(event EventSetScanData
  (params (Scanned :type Boolean))
  ;[1 1 1] Set Him to scanned
  (Variables|Default|SetScanned Scanned))

(event EventDoInteract)

(event EventObserved
  (params (BeingObserved :type Boolean)))

(fn ConstructionScript
  (bind _data (Variables|Default|GetData))
  (Utilities|Struct|SetmembersinF_ScannableData _data (.Name (Utilities|Struct|BreakF_ScannableData _data))))

(fn ReturnScanData
  (return (Variables|Default|GetData) (Variables|Character|GetMesh) (Variables|Default|GetScanned)))