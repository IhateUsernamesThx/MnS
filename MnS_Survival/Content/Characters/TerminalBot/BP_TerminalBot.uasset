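; Terminal bot character that turns its head toward a nearby player, can be scanned, and opens a terminal uplink widget on interaction.
; A looping timer set at BeginPlay drives head look, easing the Animation Blueprint's look alpha by player distance and feeding it the player's look point.
; Interacting shows the widget with UI-only input and cinematic mode.
; Observed state goes to the Blackboard, while scan data is exposed for scanning.
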(event Custom|HeadLookDetection
  (bind _abpref (Variables|Default|GetABPRef))
  ;[1 0.4233 0] Smooth Head Look
  (if (< (Transformation|GetDistanceTo (Variables|Default|GetPlayerRef)) 7e+02) ; Check player is in range
    (Variables|/Game/Characters/TerminalBot/Animations/ABP_TerminalBot.ABP_TerminalBot_C|SetHeadLookAlpha _abpref (Math|Interpolation|FInterpTo (Variables|/Game/Characters/TerminalBot/Animations/ABP_TerminalBot.ABP_TerminalBot_C|GetHeadLookAlpha _abpref) 1.0 (Utilities|Time|GetWorldDeltaSeconds) 2.0)) ; Lerp between 0 - 1 for smooth look
    (Variables|/Game/Characters/TerminalBot/Animations/ABP_TerminalBot.ABP_TerminalBot_C|SetHeadLookLocation _abpref (Transformation|GetWorldLocation (Variables|/Game/FirstPerson/Blueprints/BP_FirstPersonCharacter.BP_FirstPersonCharacter_C|GetHeadLookLoc (Variables|Default|GetPlayerRef)))) ; Set where to look at
    (elif (> (Variables|/Game/Characters/TerminalBot/Animations/ABP_TerminalBot.ABP_TerminalBot_C|GetHeadLookAlpha _abpref) 0.0) ; Check value is above 0 to prevent constant code firing
      (Variables|/Game/Characters/TerminalBot/Animations/ABP_TerminalBot.ABP_TerminalBot_C|SetHeadLookAlpha (Variables|Default|GetABPRef) (Math|Interpolation|FInterpTo (Variables|/Game/Characters/TerminalBot/Animations/ABP_TerminalBot.ABP_TerminalBot_C|GetHeadLookAlpha _abpref) 0.0 (Utilities|Time|GetWorldDeltaSeconds) 2.0)) ; Lerp between 1 - 0 for smooth look
    )))

(event EventBeginPlay
  ;[0.1886 0.4336 1] Set initial variables
  (bind _asbp_first_person_character (Utilities|Casting|CastToBP_FirstPersonCharacter (Game|GetPlayerCharacter 0)))
  (Variables|Default|SetPlayerRef _asbp_first_person_character) ; Get player reference
  (bind _asabp_terminal_bot (Utilities|Casting|CastToABP_TerminalBot (Components|SkeletalMesh|GetAnimInstance (Variables|Character|GetMesh))))
  (Variables|Default|SetABPRef _asabp_terminal_bot) ; Get Animation blueprint Reference
  (Utilities|Time|SetTimerbyEvent (EventDispatchers|CreateEvent :!event Custom|HeadLookDetection) 0.005 true) ; HeadLookTimer
  (bind _returnvalue (UserInterface|CreateWidget "/Game/UI/WB_TerminalUplink.WB_TerminalUplink_C" 0 (Transformation|GetActorLocation)))
  (Variables|Default|SetTerminalWidget _returnvalue))

(event EventObserved
  (params (BeingObserved :type Boolean))
  (AI|Components|Blackboard|SetValueasBool (AI|GetBlackboard 0) (Utilities|Name|MakeLiteralName "Observed") BeingObserved))

(event EventDoInteract
  (bind _returnvalue (Game|GetPlayerController 0))
  (UserInterface|Viewport|AddtoViewport (Variables|Default|GetTerminalWidget) 0)
  (Variables|/Script/Engine.PlayerController|SetbShowMouseCursor _returnvalue true)
  (Input|SetInputModeUIOnly _returnvalue 0 "DoNotLock" false)
  (Class|PlayerController|SetCinematicMode _returnvalue true false false true true))

(event EventSetScanData
  (params (Scanned :type Boolean))
  ;[1 1 1] Set Him to scanned
  (Variables|Default|SetScanned Scanned))

(fn ConstructionScript
  (bind _data (Variables|Default|GetData))
  (Utilities|Struct|SetmembersinF_ScannableData _data (.Name (Utilities|Struct|BreakF_ScannableData _data))))

(fn ReturnScanData
  (return (Variables|Default|GetData) (Variables|Character|GetMesh) (Variables|Default|GetScanned)))